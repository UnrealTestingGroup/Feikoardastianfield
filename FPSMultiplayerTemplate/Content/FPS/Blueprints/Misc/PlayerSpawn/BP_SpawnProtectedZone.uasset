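; Spawn protection zone actor that flags characters of other teams who enter a team's spawn area.
; On box overlap, after a short delay, it turns on a warning on any BP_BaseCharacter whose PawnTeam differs from SpawnTeam, and clears it on exit.
; The construction script sizes the box from per-instance X and Y extents with a fixed height.
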(event `self.Box.OnComponentBeginOverlap`
  (params (OverlappedComponent :type "PrimitiveComponent Object Reference") (OtherActor :type "Actor Object Reference") (OtherComp :type "PrimitiveComponent Object Reference") (OtherBodyIndex :type Integer) (bFromSweep :type Boolean) (SweepResult :type "HitResult Structure (by ref)"))
  (`KismetSystemLibrary.Delay` 0.2)
  (bind _asbp_base_character (cast `/Game/FPS/Blueprints/CharacterAndClasses/BP_BaseCharacter` OtherActor))
  (if (not (== (`/Game/FPS/Blueprints/CharacterAndClasses/BP_BaseCharacter.bPawnTeam` _asbp_base_character) (`self.SpawnTeam`)))
    (`/Game/FPS/Blueprints/CharacterAndClasses/BP_BaseCharacter.SetWarnPlayer` _asbp_base_character true)))

(event `self.Box.OnComponentEndOverlap`
  (params (OverlappedComponent :type "PrimitiveComponent Object Reference") (OtherActor :type "Actor Object Reference") (OtherComp :type "PrimitiveComponent Object Reference") (OtherBodyIndex :type Integer))
  (bind _asbp_base_character (cast `/Game/FPS/Blueprints/CharacterAndClasses/BP_BaseCharacter` OtherActor))
  (if (not (== (`/Game/FPS/Blueprints/CharacterAndClasses/BP_BaseCharacter.bPawnTeam` _asbp_base_character) (`self.SpawnTeam`)))
    (`/Game/FPS/Blueprints/CharacterAndClasses/BP_BaseCharacter.SetWarnPlayer` _asbp_base_character false)))

(fn `UserConstructionScript`
  (`BoxComponent.SetBoxExtent` (`self.Box`) (`KismetMathLibrary.MakeVector` (`self.Box_X`) (`self.Box_Y`) 300.0) true))