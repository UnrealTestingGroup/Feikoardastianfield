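; BP_StickyGrenade is a grenade that sticks to a character it hits and beeps repeatedly.
; On a Sphere hit it plays a pitched-up camera shutter sound and starts a looping timer to repeat it.
; If the hit actor is a BP_BaseCharacter, it attaches to the hit bone, keeping its world transform, and disables Sphere collision.
; This graph contains no detonation or damage logic.
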(event `self.Sphere.OnComponentHit`
  (params (HitComponent :type "PrimitiveComponent Object Reference") (OtherActor :type "Actor Object Reference") (OtherComp :type "PrimitiveComponent Object Reference") (NormalImpulse :type "Vector Structure") (Hit :type "HitResult Structure (by ref)"))
  (`GameplayStatics.PlaySoundAtLocation` "/Engine/VREditor/Sounds/UI/Camera_Shutter.Camera_Shutter" (`self.K2_GetActorLocation`) (struct) 0.2 2.0 0.0 "/Game/FPS/MusicSound/WeaponAttenuation.WeaponAttenuation" null null)
  (`KismetSystemLibrary.K2_SetTimerDelegate` (delegate `PlaySoundLoop`) 0.7 true)
  (bind _asbp_base_character (cast `/Game/FPS/Blueprints/CharacterAndClasses/BP_BaseCharacter` OtherActor))
  (`self.AttachToActor` _asbp_base_character Hit_HitBoneName)
  (`PrimitiveComponent.SetCollisionEnabled` (`self.Sphere`) "NoCollision"))

(event `PlaySoundLoop`
  (`GameplayStatics.PlaySoundAtLocation` "/Engine/VREditor/Sounds/UI/Camera_Shutter.Camera_Shutter" (`self.K2_GetActorLocation`) (struct) 0.2 2.0 0.0 "/Game/FPS/MusicSound/WeaponAttenuation.WeaponAttenuation" null null))

(event `AttachToActor`
  (params (Actor :type "Actor Object Reference") (BoneName :type Name))
  (`self.K2_AttachToActor` Actor BoneName "KeepWorld" "KeepWorld" "KeepWorld"))

(fn `UserConstructionScript`
  (`parent.UserConstructionScript`))