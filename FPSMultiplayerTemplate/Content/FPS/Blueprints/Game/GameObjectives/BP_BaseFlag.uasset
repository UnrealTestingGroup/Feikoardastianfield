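; Base capture-the-flag objective that records its spawn transform and handles character overlaps on the server only.
; A living enemy not already carrying a flag picks it up, attaching it to the character's FlagSocket.
; A living teammate's touch teleports it home, first awarding a team point through FPS_CTF_GS if they carry a flag and this one is at base.
; Scoring also sends the carried flag back to its start.
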(event `self.ReceiveBeginPlay`
  (set `self.InitialPossition` (`self.K2_GetActorLocation`))
  (set `self.InitialRotation` (`self.K2_GetActorRotation`)))

(event `self.Capsule.OnComponentBeginOverlap`
  (params (OverlappedComponent :type "PrimitiveComponent Object Reference") (OtherActor :type "Actor Object Reference") (OtherComp :type "PrimitiveComponent Object Reference") (OtherBodyIndex :type Integer) (bFromSweep :type Boolean) (SweepResult :type "HitResult Structure (by ref)"))
  (`/Engine/EditorBlueprintResources/ActorMacros.Switch Has Authority`
    (:`Authority`
      (if (not (`self.bFlagTaken`))
        (bind _asbp_base_character (cast `/Game/FPS/Blueprints/CharacterAndClasses/BP_BaseCharacter` OtherActor))
        (if (`/Game/FPS/Blueprints/CharacterAndClasses/BP_BaseCharacter.bDead` _asbp_base_character)
          _
          (elif (not (== (`/Game/FPS/Blueprints/CharacterAndClasses/BP_BaseCharacter.bPawnTeam` _asbp_base_character) (`self.Team`)))
            (if (not (`/Game/FPS/Blueprints/CharacterAndClasses/BP_BaseCharacter.bCarringFlag` _asbp_base_character))
              (`/Game/FPS/Blueprints/CharacterAndClasses/BP_BaseCharacter.OnPickupFlag` _asbp_base_character self)
              (set `self.bFlagTaken` true)
              (`/Engine/EditorBlueprintResources/StandardMacros.IsValid` _asbp_base_character
                (:`Is Valid`
                  (`self.K2_AttachToComponent` (`Character.Mesh` _asbp_base_character) "FlagSocket" "SnapToTarget" "KeepRelative" "KeepRelative"))))
            (else
              ;[1 1 1] Your Team flag
              (`self.TryToAddPoint` _asbp_base_character)
              (`self.K2_TeleportTo` (`self.InitialPossition`) (`self.InitialRotation`))
              (`self.K2_SetActorRotation` (struct))
              (`KismetSystemLibrary.Delay` 0.2)
              (`/Game/FPS/Blueprints/CharacterAndClasses/BP_BaseCharacter.OnDropFlag` _asbp_base_character)
              (set `self.bFlagTaken` false))))))))

(fn `TryToAddPoint`
  (params (Pawn :type "/Game/FPS/Blueprints/CharacterAndClasses/BP_BaseCharacter Object Reference"))
  (bind _flagref (`/Game/FPS/Blueprints/CharacterAndClasses/BP_BaseCharacter.FlagRef` Pawn))
  (if (and (`/Game/FPS/Blueprints/CharacterAndClasses/BP_BaseCharacter.bCarringFlag` Pawn) (== (`self.InitialPossition`) (`self.K2_GetActorLocation`) :`ErrorTolerance` 50.0))
    ;[1 1 1] Add points
    (bind _asfps_ctf_gs (cast `/Game/FPS/Blueprints/Game/CaptureTheFlag/FPS_CTF_GS` (`GameplayStatics.GetGameState`)))
    (`/Game/FPS/Blueprints/Game/CaptureTheFlag/FPS_CTF_GS.AddTeamPoints` _asfps_ctf_gs (`/Game/FPS/Blueprints/CharacterAndClasses/BP_BaseCharacter.bPawnTeam` Pawn))
    (`/Game/FPS/Blueprints/CharacterAndClasses/BP_BaseCharacter.DropFlag` Pawn)
    (`self.K2_SetActorLocation` _flagref (`/Game/FPS/Blueprints/Game/GameObjectives/BP_BaseFlag.InitialPossition` _flagref) false true)))

(fn `UserConstructionScript`)